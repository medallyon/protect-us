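; PU_Lib is a shared utility library for a townfolk game, offering name generation and lookup helpers.
; Random names pair a gender-matched first name with a last name, with Non-Binary randomly drawing from either male or female lists.
; Gameplay tags drive the queries, extracting Condition tags from characters and filtering all Building or BaseTownFolk actors in the world by tag.
; A final helper returns the first player controller cast to GameController.
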(fn GenerateRandomName
  (params (Gender :type Gender%20Enum :default "NewEnumerator0"))
  (bind _names (LocalVariables|GetNames))
  (bind _item (|RandomItem_2_2 (.last _names)))
  (bind _item_2 (|RandomItem (.female _names)))
  (bind _item_3 (|RandomItem_2 (.male _names)))
  (bind _returnvalue (Utilities|String|Append _item_3 " " _item))
  (bind _returnvalue_2 (Utilities|String|Append _item_2 " " _item))
  (switch Utilities|FlowControl|Switch|SwitchonGender Gender
    (:NewEnumerator0
      (return (select (Math|Random|RandomBool) _returnvalue _returnvalue_2)))
    (:NewEnumerator2
      (return _returnvalue_2))
    (:NewEnumerator1
      (return _returnvalue))))

(fn GetCharacterConditions
  (params (Character%20Tags :type Gameplay%20Tag%20Container%20Structure))
  (for _array_element (.gameplaytags Character%20Tags)
    (if (GameplayTags|MatchesTag _array_element "(TagName=\"Condition\")")
      (GameplayTags|AddGameplayTag (LocalVariables|GetConcurrent) _array_element :!class /Script/GameplayTags.BlueprintGameplayTagLibrary)))
  (return (LocalVariables|GetConcurrent)))

(fn FetchBuildings
  (params (Filter :type Gameplay%20Tag%20Structure :default "(TagName=\"Building\")") (Exact%20Match :type Boolean))
  (LocalVariables|SetTag Filter)
  (LocalVariables|SetExactMatch Exact%20Match)
  (bind _outactors (Actor|GetAllActorsOfClass 0 "/Game/_Game/Blueprints/Gameplay/Navigation/Buildings/Building.Building_C"))
  (for _array_element _outactors
    (if (GameplayTags|HasTag (Variables|/Game/_Game/Blueprints/Gameplay/Navigation/Buildings/Building.Building_C|GetBuilding%20Tags _array_element) (LocalVariables|GetTag) (LocalVariables|GetExactMatch))
      (Utilities|Array|Add (LocalVariables|GetMatching%20Buildings) _array_element)))
  (return (LocalVariables|GetMatching%20Buildings)))

(fn FetchCharacters
  (params (Filter :type Gameplay%20Tag%20Structure) (Exact%20Match :type Boolean))
  (LocalVariables|SetTag Filter)
  (LocalVariables|SetExactMatch Exact%20Match)
  (bind _outactors (Actor|GetAllActorsOfClass 0 "/Game/_Game/Blueprints/Gameplay/Navigation/Characters/BaseTownFolk.BaseTownFolk_C"))
  (for _array_element _outactors
    (if (GameplayTags|HasTag (Variables|/Game/_Game/Blueprints/Gameplay/Navigation/Characters/BaseTownFolk.BaseTownFolk_C|GetCharacter%20Tags _array_element) (LocalVariables|GetTag) (LocalVariables|GetExactMatch))
      (Utilities|Array|Add (LocalVariables|GetMatches) _array_element)))
  (return (LocalVariables|GetMatches)))

(fn FetchController
  (bind _asgame_controller (Utilities|Casting|CastToGameController (Game|GetPlayerController 0)))
  (return _asgame_controller))