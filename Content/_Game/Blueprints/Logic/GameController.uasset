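; Central game controller that runs the opening sequence, hands view to the overhead pawn, and manages HUD, menus and pausing.
; BeginPlay caches level actors, creates widgets and starts a looping intro sequence.
; The opening currently skips the TV news video, blends to the pawn, possesses it and starts the game.
; Cursor traces let clicks on townfolk open character sheets; pausing uses zero time dilation, but unpausing never removes the pause menu.
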(event Custom|Play%20Opening%20Sequence
  (|PlayOpeningSequence(dev) true))

(event Custom|Switch%20To%20Overhead%20Pawn
  (|SwitchtoPawnwithablend 5.0))

(event Custom|Start%20Game
  (Variables|Flow|SetGame%20Started true)
  (UserInterface|Viewport|AddtoViewport (Variables|Widgets|Game|GetHUD%20Widget) 0)
  (Default|CallEventGameStarted))

(event Custom|Pause%20Game
  (params (With%20Pause%20Menu :type Boolean) (With%20Background :type Boolean) (PauseTime :type Boolean))
  (|PauseGame With%20Pause%20Menu With%20Background PauseTime))

(event Custom|Unpause%20Game
  (|UnpauseGame))

(event Custom|Resume%20Game
  (CallFunction|UnpauseGame))

(event EventBeginPlay
  (Utilities|FlowControl|Sequence
    (:then_0
      (|Initialise))
    (:then_1
      (|CreateWidgets))
    (:then_2
      (|Create&StartSequencePlayer))))

(event EventTick
  (params (DeltaSeconds :type Float%20%28single-precision%29))
  (Utilities|FlowControl|Sequence
    (:then_0
      (|RecordTargetUnderCursor))))

(event Input|ActionEvents|InputActionClickLeft
  (params (Key :type Key%20Structure :default "None"))
  (:Pressed
    (|ToggleGamePaused&ToggleCharacterSheet)))

(event Input|ActionEvents|InputActionEscape
  (params (Key :type Key%20Structure :default "None"))
  (:Released
    (|ToggleGamePaused)))

(fn ConstructionScript)

(event Custom|On%20Video%20Complete
  (Utilities|FlowControl|Delay 1.0)
  (Sequencer|Player|Stop (Variables|Util|GetSequence%20Player) :!class /Script/MovieScene.MovieSceneSequencePlayer)
  (CallFunction|SwitchtoOverheadPawn))