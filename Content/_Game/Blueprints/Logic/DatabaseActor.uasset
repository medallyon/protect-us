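; DatabaseActor is a level actor that caches shared references and provides a stencil value lookup.
; On BeginPlay it stores the first Pawn_Overhead and all MovementControlPoint actors as navigation points, then creates a pause background widget without storing it or adding it to the viewport.
; GetStencilValue maps a color selection to a fixed stencil integer, with None as zero.
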(event EventBeginPlay
  (Utilities|FlowControl|Sequence
    (:then_0
      (|FetchOverheadPawn))
    (:then_1
      (bind _outactors (Actor|GetAllActorsOfClass "/Game/_Game/Blueprints/Logic/Navigation/MovementControlPoint.MovementControlPoint_C"))
      (Variables|Default|SetNavigation%20Points _outactors))
    (:then_2
      (UserInterface|CreateWidget "/Game/_Game/Blueprints/UI/PU_W_PauseBackground.PU_W_PauseBackground_C"))))

(fn ConstructionScript)

(fn GetStencilValue
  (params (Stencil :type CustomOutlineStencils%20Enum :default "NewEnumerator0"))
  (return (Utilities|Select :Index Stencil :NewEnumerator6 0 :NewEnumerator0 (Class|KismetSystemLibrary|MakeLiteralInteger 250) :NewEnumerator4 (Class|KismetSystemLibrary|MakeLiteralInteger 251) :NewEnumerator3 (Class|KismetSystemLibrary|MakeLiteralInteger 252) :NewEnumerator5 (Class|KismetSystemLibrary|MakeLiteralInteger 253) :NewEnumerator1 (Class|KismetSystemLibrary|MakeLiteralInteger 254) :NewEnumerator2 (Class|KismetSystemLibrary|MakeLiteralInteger 255))))